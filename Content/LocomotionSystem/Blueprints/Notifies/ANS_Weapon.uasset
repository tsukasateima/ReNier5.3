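; Anim notify state that forwards animation begin and end events to the item in the owner's current quick bar slot, likely a weapon.
; It finds the mesh owner's quick bar component, takes the current slot, then gets that slot's montage component, checking validity at each step.
; For every name in NotifyNames, it calls that component's notify-state begin or end event.
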(fn ReceivedNotifyBegin
  (params (MeshComp :type Skeletal%20Mesh%20Component%20Object%20Reference) (Animation :type Anim%20Sequence%20Base%20Object%20Reference) (TotalDuration :type Float%20%28single-precision%29) (EventReference :type Anim%20Notify%20Event%20Reference%20Structure%20%28by%20ref%29))
  (bind _returnvalue (Components|GetOwner MeshComp))
  (bind _returnvalue_2 (Actor|GetComponentbyClass _returnvalue "/Game/LocomotionSystem/Blueprints/Components/CT_Cmpt_QuickBar_Lite.CT_Cmpt_QuickBar_Lite_C"))
  (bind _output (Default|GetCurrentSlot _returnvalue_2))
  (bind _returnvalue_3 (Actor|GetComponentbyClass _output "/Game/LocomotionSystem/Blueprints/Components/CT_Cmpt_Montage_Lite.CT_Cmpt_Montage_Lite_C"))
  (Utilities|IsValid _returnvalue_2
    (:Is%20Valid
      (Utilities|IsValid _output
        (:Is%20Valid
          (Utilities|IsValid _returnvalue_3
            (:Is%20Valid
              (for _array_element (Variables|Default|GetNotifyNames)
                (Default|CallEventonNotifyStateBegin _returnvalue_3 _array_element))
              (return false))))))))

(fn ReceivedNotifyEnd
  (params (MeshComp :type Skeletal%20Mesh%20Component%20Object%20Reference) (Animation :type Anim%20Sequence%20Base%20Object%20Reference) (EventReference :type Anim%20Notify%20Event%20Reference%20Structure%20%28by%20ref%29))
  (bind _returnvalue (Components|GetOwner MeshComp))
  (bind _returnvalue_2 (Actor|GetComponentbyClass _returnvalue "/Game/LocomotionSystem/Blueprints/Components/CT_Cmpt_QuickBar_Lite.CT_Cmpt_QuickBar_Lite_C"))
  (bind _output (Default|GetCurrentSlot _returnvalue_2))
  (bind _returnvalue_3 (Actor|GetComponentbyClass _output "/Game/LocomotionSystem/Blueprints/Components/CT_Cmpt_Montage_Lite.CT_Cmpt_Montage_Lite_C"))
  (Utilities|IsValid _returnvalue_2
    (:Is%20Valid
      (Utilities|IsValid _output
        (:Is%20Valid
          (Utilities|IsValid _returnvalue_3
            (:Is%20Valid
              (for _array_element (Variables|Default|GetNotifyNames)
                (Default|CallEventonNotifyStateEnd _returnvalue_3 _array_element))
              (return false))))))))