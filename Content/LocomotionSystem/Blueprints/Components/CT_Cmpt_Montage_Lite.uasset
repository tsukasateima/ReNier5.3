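; Montage component that replicates animation playback and runs melee-style attack combos for the Character found as its owner's owner.
; Play and stop requests route through server to multicast events, with montage completion, blend-out, interrupt and notify callbacks re-broadcast by identifier.
; AttackCombo starts the montage chain through a server event or buffers input during an attack.
; Save Attack notifies advance buffered combos, and Reset Combo notifies clear the state.
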(event Custom|PlayComboMontage_Server
  (params (MontageToPlay :type Anim%20Montage%20Object%20Reference))
  (CallFunction|PlayComboMontage MontageToPlay))

(event Custom|ResetCombo
  (Variables|Default|SetIsAttacking? false)
  (Variables|Default|SetSaveAttack? false)
  (Variables|Default|SetComboIndex 0))

(event Custom|PlayMontage_Server
  (params (Identifier :type Name) (SkeletalMesh :type Skeletal%20Mesh%20Component%20Object%20Reference) (Montage :type Anim%20Montage%20Object%20Reference) (PlayRate :type Float%20%28single-precision%29) (StartingPosition :type Float%20%28single-precision%29) (StartingSection :type Name))
  (CallFunction|PlayMontageMulticast Identifier SkeletalMesh Montage PlayRate StartingPosition StartingSection))

(event Custom|PlayMontage_Multicast
  (params (Identifier :type Name) (SkeletalMesh :type Skeletal%20Mesh%20Component%20Object%20Reference) (Montage :type Anim%20Montage%20Object%20Reference) (PlayRate :type Float%20%28single-precision%29) (StartingPosition :type Float%20%28single-precision%29) (StartingSection :type Name))
  (bind _notifyname (Animation|Montage|PlayMontage SkeletalMesh Montage PlayRate StartingPosition StartingSection)
    (:OnCompleted
      (Default|CallEventonMontageCompleted Identifier))
    (:OnBlendOut
      (Default|CallEventonMontageBlendOut Identifier))
    (:OnInterrupted
      (Default|CallEventonMontageInterrupted Identifier))
    (:OnNotifyBegin
      (Default|CallEventonMontageNotifyBegin Identifier _notifyname))
    (:OnNotifyEnd
      (Default|CallEventonMontageNotifyEnd Identifier _notifyname))))

(event Custom|StopMontage_Server
  (params (AnimMontage :type Anim%20Montage%20Object%20Reference))
  (CallFunction|StopMontageMulticast AnimMontage))

(event Custom|AttackCombo
  (params (Character :type Character%20Object%20Reference) (Montages :type Array%20of%20Anim%20Montage%20Object%20References))
  (Variables|Default|SetCharacter Character)
  (Variables|Default|SetComboMontages Montages)
  (if (not (Variables|Default|GetIsAttacking?))
    (Variables|Default|SetIsAttacking? true)
    (CallFunction|PlayComboMontageServer (Utilities|Array|Get(acopy) (Variables|Default|GetComboMontages) (Variables|Default|GetComboIndex)))
    (else
      (Variables|Default|SetSaveAttack? true))))

(event Custom|PlayComboMontage
  (params (MontageToPlay :type Anim%20Montage%20Object%20Reference))
  (bind _notifyname (Animation|Montage|PlayMontage (Variables|/Script/Engine.Character|GetMesh (CallFunction|GetCharacter)) MontageToPlay 1.0 0.0 "Default")
    (:OnNotifyBegin
      (switch name _notifyname
        (:SaveAttack
          (if (Variables|Default|GetSaveAttack?)
            (Variables|Default|SetSaveAttack? false)
            (Variables|Default|SetComboIndex (+ (Variables|Default|GetComboIndex) 1))
            (CallFunction|PlayComboMontageServer (Utilities|Array|Get(acopy) (Variables|Default|GetComboMontages) (Variables|Default|GetComboIndex)))))
        (:ResetCombo
          (CallFunction|ResetCombo))))))

(event Custom|StopMontage_Multicast
  (params (AnimMontage :type Anim%20Montage%20Object%20Reference))
  (Animation|StopAnimMontage (CallFunction|GetCharacter) AnimMontage))

(fn GetCharacter
  (bind _as角色 (Utilities|Casting|CastToCharacter (Components|GetOwner (Components|GetOwner))))
  (return _as角色))

(fn PlayMontage
  (params (Identifier :type Name) (SkeletalMesh :type Skeletal%20Mesh%20Component%20Object%20Reference) (Montage :type Anim%20Montage%20Object%20Reference) (PlayRate :type Float%20%28single-precision%29) (StartingPosition :type Float%20%28single-precision%29) (StartingSection :type Name))
  (CallFunction|PlayMontageServer Identifier SkeletalMesh Montage PlayRate StartingPosition StartingSection))

(fn StopMontage
  (params (AnimMontage :type Anim%20Montage%20Object%20Reference))
  (CallFunction|StopMontageServer AnimMontage))