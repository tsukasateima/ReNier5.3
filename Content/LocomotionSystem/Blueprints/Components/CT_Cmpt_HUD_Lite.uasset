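; Lightweight HUD component that creates a widget for its controlled character owner and relays respawn, crosshair and grenade display requests.
; One tick after BeginPlay it adds the configured widget class to the viewport if the owner is controlled, and removes it on EndPlay.
; Show and hide functions forward to client-named events, which fire matching event dispatchers, so the component itself never updates the widget's contents.
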(event Custom|Event_OnShowRespawn_Client
  (params (Duration :type Float%20%28double-precision%29))
  (Default|CallEventonShowRespawn Duration))

(event Custom|Event_OnShowCrosshair_Client
  (Default|CallEventonShowCrosshair))

(event Custom|InitHUD
  (bind _widgetclass (Variables|Default|GetWidgetClass))
  (bind _as角色 (Utilities|Casting|CastToCharacter (Components|GetOwner)))
  (if (Class|Pawn|IsControlled _as角色)
    (Utilities|IsValid (Variables|Default|GetMainHUD)
      (:Is%20Not%20Valid
        (if (Utilities|IsValidClass _widgetclass)
          (bind _returnvalue (UserInterface|CreateWidget _widgetclass))
          (bind _output_get (Variables|Default|SetMainHUD _returnvalue))
          (UserInterface|Viewport|AddtoViewport _output_get 0))))))

(event Custom|Event_OnHideCrosshair_Client
  (Default|CallEventonHideCrosshair))

(event Custom|Event_OnShowGrenade_Client
  (Default|CallEventonShowGrenade))

(event Custom|Event_OnHideGrenade_Client
  (Default|CallEventonHideGrenade))

(event EventBeginPlay
  (Utilities|FlowControl|DelayUntilNextTick)
  (CallFunction|InitHUD))

(event EventEndPlay
  (params (EndPlayReason :type EEndPlayReason%20Enum :default "Destroyed"))
  (bind _mainhud (Variables|Default|GetMainHUD))
  (Utilities|IsValid _mainhud
    (:Is%20Valid
      (if (UserInterface|Viewport|IsinViewport _mainhud)
        (Widget|RemovefromParent (Variables|Default|GetMainHUD))))))

(fn ShowRespawn
  (params (Duration :type Float%20%28double-precision%29))
  (CallFunction|EventonShowRespawnClient Duration))

(fn ShowCrosshair
  (CallFunction|EventonShowCrosshairClient))

(fn HideCrosshair
  (CallFunction|EventonHideCrosshairClient))

(fn ShowGrenade
  (CallFunction|EventonShowGrenadeClient))

(fn HideGrenade
  (CallFunction|EventonHideGrenadeClient))